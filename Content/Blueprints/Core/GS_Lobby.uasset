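; GS_Lobby is a lobby Blueprint, apparently a GameState, whose only logic is a leftover debug readout of player ready status.
; That graph has no event driving it, so it never runs.
; It would loop over PlayerArray, cast each entry to PlayerStateTest, and briefly print the one-based player number and ReadyStatus.
; The authority and remote branches print identical messages, and the construction script is empty.
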(fn ConstructionScript)