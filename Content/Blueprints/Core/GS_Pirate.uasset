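; Game State for a Pirate (red) versus Navy (blue) team match, handling usernames and the win condition.
; On BeginPlay it copies the Game Instance username into each PlayerStateTest whose PlayerNumber matches its PlayerArray index.
; CheckScore tests red, then blue score for equality with WinLimit.
; On a win, it replaces widgets on each TestDummy pawn, fetched by player index, with the winning team's screen.
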(event Custom|CheckScore
  (if (== (Variables|Default|GetRedScore) (Variables|Default|GetWinLimit))
    (Variables|Default|SetRedWins? true)
    (for (_ _array_index) (Variables|Default|GetPlayerArray) :!label _label
      (bind _astest_dummy (Utilities|Casting|CastToTestDummy (Game|Player|GetPlayerPawn _array_index)))
      (Default|DestroyAllWidgets _astest_dummy)
      (Default|CreateWidgetforWinning _astest_dummy (select (Variables|Default|GetRedWins?) "Pirate Wins!" "Navy Wins!") (Variables|Default|GetRedWins?)))
    (elif (== (Variables|Default|GetBlueScore) (Variables|Default|GetWinLimit))
      (Variables|Default|SetRedWins? false)
      (goto _label))))

(event EventBeginPlay
  (for (_array_element _array_index) (Variables|Default|GetPlayerArray)
    (bind _asgame_instance_test (Utilities|Casting|CastToGameInstanceTest (Game|GetGameInstance)))
    (bind _asplayer_state_test (Utilities|Casting|CastToPlayerStateTest _array_element))
    (if (== (Variables|/Game/Blueprints/Core/PlayerStateTest.PlayerStateTest_C|GetPlayer%20Number _asplayer_state_test) _array_index)
      (Variables|/Game/Blueprints/Core/PlayerStateTest.PlayerStateTest_C|SetUsername%20%28PlayerState%29 _asplayer_state_test (Variables|/Game/Blueprints/Core/GameInstanceTest.GameInstanceTest_C|GetUsername%20%28GameInstance%29 _asgame_instance_test)))))

(fn ConstructionScript)