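; Lobby game mode that numbers joining players and server-travels everyone to TestMap as a listen server once its ready check passes.
; PostLogin sets each PlayerStateTest's PlayerNumber to the last PlayerArray index.
; CheckPlayerReady copies ready flags and compares array lengths, so unready players below the highest ready index can slip through.
; ReadyToStartMatch returns false, and the default pawn class override returns no class.
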(event Custom|DIsplayPlayerName
  (params (bPickA :type Boolean))
  ;[1 1 1] To check if all of the players are ready
  (for _array_element (Variables|/Script/Engine.GameState|GetPlayerArray (Game|GetGameState))
    (Development|PrintString (Utilities|String|Append (Utilities|String|SelectString "BEFORE TRAVEL : " "AFTER TRAVEL : " bPickA) (Utilities|GetDisplayName _array_element)) true true "(R=0.000000,G=0.660000,B=1.000000,A=1.000000)" 1e+01)))

(event Custom|CheckPlayerReady
  (bind _readystatuses (Variables|Default|GetReadyStatuses))
  (bind _returnvalue (Utilities|Array|Length _readystatuses))
  ;[1 1 1] To check if all of the players are ready
  (Utilities|FlowControl|Sequence
    (:then_0
      (for (_array_element _array_index) (Variables|/Script/Engine.GameState|GetPlayerArray (Game|GetGameState))
        (bind _asplayer_state_test (Utilities|Casting|CastToPlayerStateTest _array_element))
        (Utilities|Array|SetArrayElem (Variables|Default|GetReadyStatuses) _array_index (Variables|/Game/Blueprints/Core/PlayerStateTest.PlayerStateTest_C|GetReadyStatus _asplayer_state_test) true)))
    (:then_1
      (for (_array_element_2 _array_index_2) (Variables|Default|GetReadyStatuses)
        (if (Math|Boolean|Equal(Boolean) _array_element_2 true)
          (Utilities|Array|SetArrayElem (Variables|Default|GetCheckForReady) _array_index_2 true true)))
      (if (and (== _returnvalue (Utilities|Array|Length (Variables|Default|GetCheckForReady))) (!= _returnvalue 0))
        (CallFunction|DIsplayPlayerName true)
        (Development|ExecuteConsoleCommand "ServerTravel TestMap?listen")
        (else
          (Development|PrintString "EVERYONE IS NOT READY!"))))))

(event EventPostLogin
  (params (NewPlayer :type Player%20Controller%20Object%20Reference))
  ;[1 1 1] Post login
  (Networking|SwitchHasAuthority
    (:Authority
      (bind _asplayer_state_test (Utilities|Casting|CastToPlayerStateTest (Variables|/Script/Engine.Controller|GetPlayerState NewPlayer)))
      (Variables|/Game/Blueprints/Core/PlayerStateTest.PlayerStateTest_C|SetPlayer%20Number _asplayer_state_test (Utilities|Array|LastIndex (Variables|/Script/Engine.GameState|GetPlayerArray (Game|GetGameState)))))))

(fn ConstructionScript)

(fn ReadytoStartMatch
  (return false))

(fn GetDefaultPawnClassforController
  (params (InController :type Controller%20Object%20Reference))
  (return 0))