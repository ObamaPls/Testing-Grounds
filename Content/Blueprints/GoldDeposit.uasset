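; GoldDeposit is a team-owned deposit zone that scores the GoldUnit actors inside its GoldTrigger volume.
; Entering gold adds a point and leaving gold removes one, with each unit's HasCounted flag guarding against double counting.
; AddScore applies the change to RedScore or BlueScore on GS_Pirate according to TeamOwner, then calls CheckScore on that game state.
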(event OnComponentBeginOverlap(GoldTrigger)
  (params (OtherActor :type Actor%20Object%20Reference) (OtherComp :type Primitive%20Component%20Object%20Reference) (OtherBodyIndex :type Integer) (bFromSweep :type Boolean) (SweepResult :type Hit%20Result%20Structure%20%28by%20ref%29))
  (bind _asgold_unit (Utilities|Casting|CastToGoldUnit OtherActor))
  (if (not (Variables|/Game/Blueprints/GoldUnit.GoldUnit_C|GetHasCounted _asgold_unit))
    (Variables|/Game/Blueprints/GoldUnit.GoldUnit_C|SetHasCounted _asgold_unit true)
    (Utilities|AddScore 1)))

(event OnComponentEndOverlap(GoldTrigger)
  (params (OtherActor :type Actor%20Object%20Reference) (OtherComp :type Primitive%20Component%20Object%20Reference) (OtherBodyIndex :type Integer))
  (bind _asgold_unit (Utilities|Casting|CastToGoldUnit OtherActor))
  (if (Variables|/Game/Blueprints/GoldUnit.GoldUnit_C|GetHasCounted _asgold_unit)
    (Variables|/Game/Blueprints/GoldUnit.GoldUnit_C|SetHasCounted _asgold_unit false)
    (Utilities|AddScore -1)))

(fn ConstructionScript)