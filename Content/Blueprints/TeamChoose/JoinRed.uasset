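; JoinRed is a team-selection trigger that puts an overlapping TestDummy on a team, presumably red going by its name.
; On entering TeamChooseRange, it sets Team on the dummy's PlayerStateTest, calls JoinTeam, then moves it to the RedSpawnLoc of the first DeathZ actor found.
; End overlap does nothing, as the logic that would set a different team value is disconnected.
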(event OnComponentBeginOverlap(TeamChooseRange)
  (params (OtherActor :type Actor%20Object%20Reference) (OtherComp :type Primitive%20Component%20Object%20Reference) (OtherBodyIndex :type Integer) (bFromSweep :type Boolean) (SweepResult :type Hit%20Result%20Structure%20%28by%20ref%29))
  (bind _astest_dummy (Utilities|Casting|CastToTestDummy OtherActor))
  (bind _asplayer_state_test (Utilities|Casting|CastToPlayerStateTest (Variables|/Script/Engine.Pawn|GetPlayerState _astest_dummy)))
  (Variables|/Game/Blueprints/Core/PlayerStateTest.PlayerStateTest_C|SetTeam _asplayer_state_test "NewEnumerator0")
  (Default|JoinTeam _astest_dummy)
  (bind _outactors (Actor|GetAllActorsOfClass "/Game/Blueprints/DeathZ.DeathZ_C"))
  (Transformation|SetActorLocation _astest_dummy (Transformation|GetWorldLocation (Variables|/Game/Blueprints/DeathZ.DeathZ_C|GetRedSpawnLoc (Utilities|Array|Get(acopy) _outactors))) false false))

(event OnComponentEndOverlap(TeamChooseRange)
  (params (OtherActor :type Actor%20Object%20Reference) (OtherComp :type Primitive%20Component%20Object%20Reference) (OtherBodyIndex :type Integer)))

(fn ConstructionScript)