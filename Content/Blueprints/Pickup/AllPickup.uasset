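; Pickup actor that cycles randomly between Health, SpeedUp and Invulnerable, floating and spinning on a timeline.
; Construction picks an initial type, then an authority-only looping timer rerolls it and swaps mesh and material.
; Duration is set at construction and BeginPlay, not on rerolls.
; On overlap it passes type and duration to TestDummy, records its location in the PickupLocation actor, then destroys itself.
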(event OnComponentBeginOverlap(PickupCollision)
  (params (OtherActor :type Actor%20Object%20Reference) (OtherComp :type Primitive%20Component%20Object%20Reference) (OtherBodyIndex :type Integer) (bFromSweep :type Boolean) (SweepResult :type Hit%20Result%20Structure%20%28by%20ref%29))
  (bind _pickupmaster (Variables|Default|GetPickupMaster))
  ;[1 1 1] Trigger
  (bind _astest_dummy (Utilities|Casting|CastToTestDummy OtherActor))
  (Default|PickupEvent _astest_dummy (Variables|Default|GetPickupValue) (Variables|Default|GetDuration))
  (Utilities|Array|Add (Variables|/Game/Blueprints/Pickup/PickupLocation.PickupLocation_C|GetPickUpLoc _pickupmaster) (Transformation|GetWorldLocation (Variables|Default|GetRoot)))
  (Variables|/Game/Blueprints/Pickup/PickupLocation.PickupLocation_C|SetInitLocation _pickupmaster "0, 0, 0")
  (Actor|DestroyActor))

(event Custom|PickupAnimation
  (bind _inittransform (Variables|Default|GetInitTransform))
  (bind (_location _rotation) (Math|Transform|BreakTransform _inittransform))
  (bind (_roll _pitch _yaw) (Math|Rotator|BreakRotator _rotation))
  ;[1 1 1] Pickup floating animation
  (bind (_direction _floating _spin) (Timeline|Animation Play)
    (:Update
      (Transformation|SetActorTransform (Math|Transform|MakeTransform (Math|Vector|Lerp(Vector) _location (+ _location "0, 0,20.000000") _floating) (Math|Rotator|Lerp(Rotator) "0, 0, 0" (Math|Rotator|MakeRotator _roll _pitch (+ _yaw 3.6e+02)) _spin))))))

(event Custom|ChangeMesh
  (params (Index :type PickUpEnum%20Enum))
  (bind _pickupcollision (Variables|Default|GetPickupCollision))
  (Components|StaticMesh|SetStaticMesh _pickupcollision (Utilities|Select :Index Index :NewEnumerator0 "/Game/Meshes/Powerup/SM_Health.SM_Health" :NewEnumerator1 "/Game/Meshes/Powerup/SM_Speed.SM_Speed" :NewEnumerator2 "/Game/Meshes/Powerup/SM_Invulnerability.SM_Invulnerability"))
  (Rendering|Material|SetMaterial _pickupcollision 0 (Utilities|Select :Index Index :NewEnumerator0 "/Game/Materials/Mat_HealthPickup.Mat_HealthPickup" :NewEnumerator1 "/Game/Materials/Mat_SpeedPickup.Mat_SpeedPickup" :NewEnumerator2 "/Game/Materials/Mat_InvulnerablePickup.Mat_InvulnerablePickup")))

(event Custom|EnumChangeServer
  (CallFunction|EnumMulticast))

(event Custom|EnumMulticast
  (Networking|SwitchHasAuthority ; Need to spawn only in server
    (:Authority
      (Utilities|Time|SetTimerbyFunctionName 0 "ChangeEnum" 2.0 true))))

(event EventBeginPlay
  (CallFunction|SetupPickupData)
  (CallFunction|EnumChangeServer)
  (bind _outactors (Actor|GetAllActorsOfClass "/Game/Blueprints/Pickup/PickupLocation.PickupLocation_C"))
  (Variables|Default|SetPickupMaster (Utilities|Array|Get(acopy) _outactors))
  (CallFunction|PickupAnimation)
  (Variables|Default|SetInitTransform (Transformation|GetActorTransform)))

(event EventTick
  (params (DeltaSeconds :type Float%20%28single-precision%29)))

(fn ConstructionScript
  (bind _output_get (Variables|Default|SetPickupValue (Utilities|Select :Index (Math|Conversions|ToByte(Integer) (Math|Random|RandomInteger 2)) :Option%200 "NewEnumerator0" :Option%201 "NewEnumerator1" :Option%202 "NewEnumerator2")))
  (Rendering|Components|TextRender|SetText (Variables|Default|GetTextRender) (Utilities|Text|ToText(String) (Utilities|String|EnumtoString _output_get)))
  (CallFunction|SetupPickupData))

(fn SetupPickupData
  (switch Utilities|FlowControl|Switch|SwitchonPickUpEnum (Variables|Default|GetPickupValue)
    (:NewEnumerator1
      (Variables|Default|SetDuration 1e+01))
    (:NewEnumerator2
      (Variables|Default|SetDuration 5.0))))

(fn ChangeEnum
  (bind _output_get (Variables|Default|SetPickupValue (Utilities|Select :Index (Math|Conversions|ToByte(Integer) (Math|Random|RandomInteger 3)) :Option%200 "NewEnumerator0" :Option%201 "NewEnumerator1" :Option%202 "NewEnumerator2")))
  (CallFunction|ChangeMesh _output_get)
  (return))