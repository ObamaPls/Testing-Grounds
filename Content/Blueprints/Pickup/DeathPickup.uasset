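; DeathPickup is a floating health pickup that heals a TestDummy on overlap, then destroys itself.
; The heal amount is selected from fixed tiers by HealthValue.
; On BeginPlay it briefly delays enabling overlap events on PickupCollision so HealthValue can be set up first.
; A timeline drives the bob and spin by lerping the actor transform from its cached initial transform.
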(event OnComponentBeginOverlap(Trigger)
  (params (OtherActor :type Actor%20Object%20Reference) (OtherComp :type Primitive%20Component%20Object%20Reference) (OtherBodyIndex :type Integer) (bFromSweep :type Boolean) (SweepResult :type Hit%20Result%20Structure%20%28by%20ref%29))
  (bind _astest_dummy (Utilities|Casting|CastToTestDummy OtherActor))
  (Default|HealAmount _astest_dummy (Utilities|Select :Index (Variables|Default|GetHealthValue) :NewEnumerator0 1e+01 :NewEnumerator1 35.0 :NewEnumerator2 5e+01))
  (Actor|DestroyActor))

(event Custom|PickupAnimation
  (bind _inittransform (Variables|Default|GetInitTransform))
  (bind (_location _rotation) (Math|Transform|BreakTransform _inittransform))
  (bind (_roll _pitch _yaw) (Math|Rotator|BreakRotator _rotation))
  ;[1 1 1] Pickup floating animation
  (bind (_direction _floating _spin) (Timeline|Animation Play)
    (:Update
      (Transformation|SetActorTransform (Math|Transform|MakeTransform (Math|Vector|Lerp(Vector) _location (+ _location "0, 0,20.000000") _floating) (Math|Rotator|Lerp(Rotator) "0, 0, 0" (Math|Rotator|MakeRotator _roll _pitch (+ _yaw 3.6e+02)) _spin))))))

(event EventBeginPlay
  (CallFunction|PickupAnimation)
  (Variables|Default|SetInitTransform (Transformation|GetActorTransform))
  (Utilities|FlowControl|Delay 0.2) ; To wait for the setting up of HealthValue in TestDummy
  (Variables|/Script/Engine.PrimitiveComponent|SetbGenerateOverlapEvents (Variables|Default|GetPickupCollision) true))

(fn ConstructionScript)