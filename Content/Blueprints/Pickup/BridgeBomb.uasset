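; BridgeBomb is a pickup that destroys every Bridge in the level when a TestDummy overlaps its trigger.
; On overlap it hides the trigger and disables its collision, then passes each valid Bridge and its array index to GM_Pirate's DestroyBridge.
; It destroys itself only after the loop, since destroying it first could leave a bridge standing.
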(event OnComponentBeginOverlap(Trigger)
  (params (OtherActor :type Actor%20Object%20Reference) (OtherComp :type Primitive%20Component%20Object%20Reference) (OtherBodyIndex :type Integer) (bFromSweep :type Boolean) (SweepResult :type Hit%20Result%20Structure%20%28by%20ref%29))
  (bind _trigger (Variables|Default|GetTrigger))
  (Utilities|Casting|CastToTestDummy OtherActor)
  (Rendering|SetVisibility _trigger false false) ; Hiding it because if destroyed first, there's a chance that a bridge not being destroyed
  (Collision|SetCollisionEnabled _trigger "NoCollision")
  (bind _outactors (Actor|GetAllActorsOfClass "/Game/Blueprints/BridgeSystem/Bridge.Bridge_C"))
  (for (_array_element _array_index) _outactors
    (Utilities|IsValid _array_element
      (:Is%20Valid
        (bind _asgm_pirate (Utilities|Casting|CastToGM_Pirate (Game|GetGameMode)))
        (Default|DestroyBridge _asgm_pirate _array_element _array_index))))
  (Actor|DestroyActor))

(fn ConstructionScript)