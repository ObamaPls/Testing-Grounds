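; GoldUnit is a droppable gold object that stores a value and is launched with a velocity impulse.
; Trace detect and reset events toggle an outline, and a player trace reset event clears the last traced actor on the TestDummy player.
; Its first physical hit fires a one-second particle burst, and overlapping a KillZ destroys it.
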(event OnComponentHit(Gold)
  (params (OtherActor :type Actor%20Object%20Reference) (OtherComp :type Primitive%20Component%20Object%20Reference) (NormalImpulse :type Vector :default "0, 0, 0") (Hit :type Hit%20Result%20Structure%20%28by%20ref%29))
  (bind _particlesystem (Variables|Default|GetParticleSystem))
  (Utilities|FlowControl|DoOnce false
    (:Completed
      (Components|Activation|Activate _particlesystem false)
      (Utilities|FlowControl|Delay 1.0)
      (Components|Activation|Deactivate _particlesystem))))

(event OnComponentBeginOverlap(Gold)
  (params (OtherActor :type Actor%20Object%20Reference) (OtherComp :type Primitive%20Component%20Object%20Reference) (OtherBodyIndex :type Integer) (bFromSweep :type Boolean) (SweepResult :type Hit%20Result%20Structure%20%28by%20ref%29))
  (Utilities|Casting|CastToKillZ OtherActor)
  (Actor|DestroyActor))

(event Custom|TraceDetect
  ;[1 1 1] Set Outline
  (Rendering|SetVisibility (Variables|Default|GetOutline) true false))

(event Custom|TraceReset
  ;[1 1 1] Set Outline
  (Rendering|SetVisibility (Variables|Default|GetOutline) false false))

(event Custom|Dropped
  (params (Impulse :type Vector) (Value :type Integer))
  (Physics|AddImpulse (Variables|Default|GetGold) Impulse "None" true)
  (Variables|Default|SetGoldValue Value))

(event Custom|PlayerTraceReset
  (bind _astest_dummy (Utilities|Casting|CastToTestDummy (Variables|Default|GetPlayerReference)))
  (Variables|/Game/Blueprints/TestDummy.TestDummy_C|SetLastActorTraced _astest_dummy 0))

(fn ConstructionScript)