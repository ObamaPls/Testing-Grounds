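; RopeSpline is a rope Blueprint that builds spline mesh segments along its Spline component in the construction script.
; It adds one spline mesh component per spline point, including the last, bending each from that point to the next using local locations and tangents.
; Each component is added with manual attachment, then attached to the spline with snap to target, including scale.
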(fn ConstructionScript
  (bind _spline (Variables|Default|GetSpline))
  (bind _spline_2 (Variables|Default|GetSpline))
  (for _index (range 0 (- (Spline|GetNumberOfSplinePoints _spline_2) 1))
    (bind _returnvalue (AddComponent|AddSplineMeshComponent true (Math|Conversions|ToTransform(Vector) (Spline|GetLocationatSplinePoint _spline_2 _index "Local"))))
    (SplineMesh|SetStartandEnd _returnvalue (.Location (Spline|GetLocationandTangentatSplinePoint _spline _index "Local")) (.Tangent (Spline|GetLocationandTangentatSplinePoint _spline _index "Local")) (.Location (Spline|GetLocationandTangentatSplinePoint _spline (+ _index 1) "Local")) (.Tangent (Spline|GetLocationandTangentatSplinePoint _spline (+ _index 1) "Local")) :!class /Script/Engine.SplineMeshComponent)
    (Class|SceneComponent|Attachto _returnvalue (Variables|Default|GetSpline) "None" "SnapToTargetIncludingScale" true)))