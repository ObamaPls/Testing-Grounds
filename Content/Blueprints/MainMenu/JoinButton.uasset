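; JoinButton is a clickable main menu Blueprint that opens the Join Game UI.
; On BeginPlay it creates the WIdget_JoinGame widget for the first player controller, stores it and adds it to the viewport hidden.
; Clicking its static mesh switches input to UI-only focused on that widget and makes it visible.
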(event OnClicked(StaticMeshComponent)
  (params (TouchedComponent :type Primitive%20Component%20Object%20Reference))
  (bind _widget_joingame (Variables|Default|GetWidget_JoinGame))
  (Input|SetInputModeUIOnly 0 _widget_joingame false)
  (Widget|SetVisibility _widget_joingame "Visible"))

(event EventBeginPlay
  (|CallParentFunction)
  (bind _returnvalue (UserInterface|CreateWidget "/Game/Blueprints/Widgets/WIdget_JoinGame.WIdget_JoinGame_C" (Game|GetPlayerController 0)))
  (Variables|Default|SetWidget_JoinGame _returnvalue)
  (Widget|SetVisibility _returnvalue "Hidden")
  (UserInterface|Viewport|AddtoViewport _returnvalue 0))

(fn ConstructionScript
  (|CallParentFunction))