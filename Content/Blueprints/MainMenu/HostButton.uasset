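; A clickable 3D main-menu button that hosts a multiplayer game.
; Clicking its static mesh removes all widgets and runs a console command that opens PlayLevel_Main as a listen server.
; Hovering slightly enlarges the mesh on X and Y from the scale cached at BeginPlay, and leaving restores it.
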(event OnEndCursorOver(StaticMeshComponent)
  (params (TouchedComponent :type Primitive%20Component%20Object%20Reference))
  (Transformation|SetWorldScale3D (Variables|Debug|GetStaticMeshComponent) (Variables|Default|GetInitial%20Size)))

(event OnClicked(StaticMeshComponent)
  (params (TouchedComponent :type Primitive%20Component%20Object%20Reference))
  (Viewport|RemoveAllWidgets)
  (Development|ExecuteConsoleCommand "open PlayLevel_Main?listen" (Game|GetPlayerController 0)))

(event OnBeginCursorOver(StaticMeshComponent)
  (params (TouchedComponent :type Primitive%20Component%20Object%20Reference))
  (Transformation|SetWorldScale3D (Variables|Debug|GetStaticMeshComponent) (+ (Variables|Default|GetInitial%20Size) "0.100000,0.100000, 0")))

(event EventBeginPlay
  (Variables|Default|SetInitial%20Size (Transformation|GetWorldScale (Variables|Debug|GetStaticMeshComponent))))

(fn ConstructionScript)