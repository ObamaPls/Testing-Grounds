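; LobbyPawn is the lobby pawn, which creates the Lobby widget on BeginPlay, shows the mouse cursor and reveals the host Start button under authority.
; Tick copies the first player controller's PlayerNumber from PlayerStateTest into GameInstanceTest.
; GetUsername returns the name from its player state, and the B key prints both player numbers for debugging.
; An IsLocallyControlled check before widget creation is left unconnected.
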(event EventBeginPlay
  (bind _returnvalue (Game|GetPlayerController 0))
  (bind _returnvalue_2 (UserInterface|CreateWidget "/Game/Blueprints/Widgets/Lobby.Lobby_C" _returnvalue)) ; This widget will be called everytime a new player pops up
  (UserInterface|Viewport|AddtoViewport _returnvalue_2 0)
  (Variables|Default|SetLobbyWidgetReference _returnvalue_2)
  (Variables|/Script/Engine.PlayerController|SetbShowMouseCursor _returnvalue true)
  (Variables|/Script/Engine.PlayerController|SetbEnableMouseOverEvents _returnvalue true)
  (Networking|SwitchHasAuthority
    (:Authority
      (Widget|SetIsEnabled (Variables|/Game/Blueprints/Widgets/Lobby.Lobby_C|GetStartButtonForHost (Variables|Default|GetLobbyWidgetReference)) true)
      (Widget|SetVisibility (Variables|/Game/Blueprints/Widgets/Lobby.Lobby_C|GetStartButtonForHost (Variables|Default|GetLobbyWidgetReference)) "Visible"))))

(event EventTick
  (params (DeltaSeconds :type Float%20%28single-precision%29))
  (bind _asplayer_state_test (Utilities|Casting|CastToPlayerStateTest (Variables|/Script/Engine.Controller|GetPlayerState (Game|GetPlayerController 0))))
  (bind _asgame_instance_test (Utilities|Casting|CastToGameInstanceTest (Game|GetGameInstance)))
  (Variables|/Game/Blueprints/Core/GameInstanceTest.GameInstanceTest_C|SetPlayerNumber _asgame_instance_test (Variables|/Game/Blueprints/Core/PlayerStateTest.PlayerStateTest_C|GetPlayer%20Number _asplayer_state_test)))

(event Input|KeyboardEvents|B
  (params (Key :type Key%20Structure :default "AnyKey"))
  (:Pressed
    (bind _asgame_instance_test (Utilities|Casting|CastToGameInstanceTest (Game|GetGameInstance)))
    (bind _asplayer_state_test (Utilities|Casting|CastToPlayerStateTest (Variables|GetPlayerState)))
    (Development|PrintString (Utilities|String|Append "PSN :" (Utilities|String|ToString(Integer) (Variables|/Game/Blueprints/Core/PlayerStateTest.PlayerStateTest_C|GetPlayer%20Number _asplayer_state_test)) " | GIN : " (Utilities|String|ToString(Integer) (Variables|/Game/Blueprints/Core/GameInstanceTest.GameInstanceTest_C|GetPlayerNumber _asgame_instance_test))))))

(fn ConstructionScript)

(fn GetUsername
  (bind _asplayer_state_test (Utilities|Casting|CastToPlayerStateTest (Variables|GetPlayerState)))
  (return (Variables|/Game/Blueprints/Core/PlayerStateTest.PlayerStateTest_C|GetUsername%20%28PlayerState%29 _asplayer_state_test)))