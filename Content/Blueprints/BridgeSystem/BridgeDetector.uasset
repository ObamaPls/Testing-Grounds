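; Bridge detector actor that overlays a 2D cell grid on a box detection zone; only the grid math is implemented here.
; Construction derives cell counts from the zone extent, then resizes the box and optionally draws one-shot debug cells.
; Helpers convert between world points, grid coordinates and flattened indices, measured from a pivot relative to the actor.
; World-to-grid conversion divides both axes by the X cell size.
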(event EventBeginPlay)

(fn ConstructionScript
  (bind _boxsize (Variables|Default|GetBoxSize))
  (bind _detectionzone (Variables|Components|GetDetectionZone))
  (bind (_x _y) (Math|Vector2D|BreakVector2D _boxsize))
  (bind _boxextent (Variables|/Script/Engine.BoxComponent|GetBoxExtent _detectionzone))
  (bind _returnvalue (* _boxextent 2.0))
  (bind (_x_2 _y_2) (Math|Vector|BreakVector _returnvalue))
  (Utilities|FlowControl|Sequence
    (:then_0
      (Variables|Default|SetMaxY (+ (Math|Float|Truncate (/ _y_2 (Variables|Default|GetGridSizeY))) 1))
      (Variables|Default|SetMaxX (+ (Math|Float|Truncate (/ _x_2 (Variables|Default|GetGridSizeX))) 1)))
    (:then_1
      (Components|Box|SetBoxExtent (Variables|Components|GetDetectionZone) (Math|Vector|MakeVector _x _y 32.0) true))
    (:then_2
      (CallFunction|DebugGridLocation))))

(fn DebugGridLocation
  (bind (_x _y) (CallFunction|GetGridPivotWorldLoc))
  (if (Variables|Default|GetDebug)
    (for _index (range 0 (- (Math|Float|Truncate (Math|Float|Absolute(Float) (/ (* (.X (Math|Vector|BreakVector (Variables|/Script/Engine.BoxComponent|GetBoxExtent (Variables|Components|GetDetectionZone)))) 2.0) (Variables|Default|GetGridSizeX)))) 1))
      (Rendering|Debug|DrawDebugBox (Math|Vector|MakeVector (+ (* (Math|Conversions|ToFloat(Integer) _index) (Variables|Default|GetGridSizeX)) _x) _y (.Z (Math|Vector|BreakVector (Transformation|GetActorLocation)))) (Math|Vector|MakeVector (Variables|Default|GetGridSizeX) (Variables|Default|GetGridSizeY) 2e+01) "(R=1.000000,G=0.000000,B=0.975927,A=1.000000)" "0, 0, 0" 3.0)
      (for _index_2 (range 0 (- (Math|Float|Truncate (Math|Float|Absolute(Float) (/ (* (.Y (Math|Vector|BreakVector (Variables|/Script/Engine.BoxComponent|GetBoxExtent (Variables|Components|GetDetectionZone)))) 2.0) (Variables|Default|GetGridSizeY)))) 1))
        (Rendering|Debug|DrawDebugBox (Math|Vector|MakeVector (+ (* (Math|Conversions|ToFloat(Integer) _index) (Variables|Default|GetGridSizeX)) _x) (+ (* (Math|Conversions|ToFloat(Integer) _index_2) (Variables|Default|GetGridSizeY)) _y) (.Z (Math|Vector|BreakVector (Transformation|GetActorLocation)))) (Math|Vector|MakeVector (Variables|Default|GetGridSizeX) (Variables|Default|GetGridSizeY) 2e+01) "(R=1.000000,G=0.000000,B=0.727159,A=1.000000)" "0, 0, 0" 3.0)))
    (Variables|Default|SetDebug false)))

(fn GetGridPivotWorldLoc
  (bind _returnvalue (Transformation|GetActorLocation))
  (bind _gridpivot (Variables|Default|GetGridPivot))
  (bind _returnvalue_2 (+ _gridpivot _returnvalue))
  (bind (_x _y) (Math|Vector|BreakVector _returnvalue_2))
  (return _x _y))

(fn ConvertPointtoGrid
  (params (World%20Location :type Vector))
  (bind (_x _y) (CallFunction|GetGridPivotWorldLoc))
  (bind (_x_2 _y_2) (Math|Vector|BreakVector World%20Location))
  (return (Math|Vector2D|MakeVector2D (Math|Conversions|ToFloat(Integer) (Math|Float|Truncate (/ (- _x_2 _x) (Variables|Default|GetGridSizeX)))) (Math|Conversions|ToFloat(Integer) (Math|Float|Truncate (/ (- _y_2 _y) (Variables|Default|GetGridSizeX)))))))

(fn DebugLocation
  (params (Loc :type Vector%202D%20Structure)))

(fn ConvertGridtoPoint
  (params (GridLocation :type Vector%202D%20Structure) (Use%20CenterPoint :type Boolean))
  (bind (_x _y) (Math|Vector2D|BreakVector2D GridLocation))
  (bind (_x_2 _y_2) (CallFunction|GetGridPivotWorldLoc))
  (bind _gridsizex (Variables|Default|GetGridSizeX))
  (bind _detectionzone (Variables|Components|GetDetectionZone))
  (bind _gridsizey (Variables|Default|GetGridSizeY))
  (bind _returnvalue (Transformation|GetWorldLocation _detectionzone))
  (bind _returnvalue_2 (* _y _gridsizey))
  (bind _returnvalue_3 (* _x _gridsizex))
  (bind _z (Math|Vector|BreakVector _returnvalue))
  (bind _returnvalue_4 (+ _returnvalue_2 _y_2))
  (bind _returnvalue_5 (+ _returnvalue_3 _x_2))
  (bind _returnvalue_6 (Math|Vector|MakeVector _returnvalue_5 _returnvalue_4 _z))
  (if Use%20CenterPoint
    (return (+ _returnvalue_6 (Math|Vector|MakeVector (/ (Variables|Default|GetGridSizeX) 2.0) (/ (Variables|Default|GetGridSizeY) 2.0) 0.0)))
    (else
      (return _returnvalue_6))))

(fn ConvertPointtoInt
  (params (Point :type Vector%202D%20Structure))
  (bind (_x _y) (Math|Vector2D|BreakVector2D Point))
  (return (+ (* (Math|Float|Truncate _x) (Variables|Default|GetMaxY)) (Math|Float|Truncate _y))))