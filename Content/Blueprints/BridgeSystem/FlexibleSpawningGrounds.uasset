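; Bridge-system actor that fills a flat rectangular area, from its origin to EndLocation, with a grid of Trigger child actors.
; Spawning uses nested X and Y loops to add child actor components at Distance intervals.
; The construction script zeroes EndLocation's Z and previews the grid when LevelDesignMode is on.
; BeginPlay builds the grid only with that mode off, otherwise printing a reminder to disable it.
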(event EventBeginPlay
  (if (Variables|Default|GetLevelDesignMode?)
    (Development|PrintString "PLEASE TURN OFF LEVEL DESIGN MODE")
    (else
      (CallFunction|Spawning))))

(event EventTick
  (params (DeltaSeconds :type Float%20%28single-precision%29)))

(fn ConstructionScript
  (Utilities|FlowControl|Sequence
    (:then_0
      (Variables|Default|SetEnd%20Location (Math|Vector|MakeVector (.X (Math|Vector|BreakVector (Variables|Default|GetEnd%20Location))) (.Y (Math|Vector|BreakVector (Variables|Default|GetEnd%20Location))) 0.0)))
    (:then_1
      (if (Variables|Default|GetLevelDesignMode?)
        (CallFunction|Spawning)))))

(fn Spawning
  ;[1 1 1] Optional
  (if (> (Math|Vector|VectorLengthSquared (Variables|Default|GetEnd%20Location)) 0.0)
    (Utilities|FlowControl|Sequence
      (:then_0
        (for _index (range 0 (Math|Float|Truncate (/ (.X (Math|Vector|BreakVector (Variables|Default|GetEnd%20Location))) (Variables|Default|GetDistance))))
          ;[1 1 1] Spawns and sets the object based on the location and increments
          (bind _returnvalue (AddComponent|AddChildActorComponent false (Math|Transform|MakeTransform (Math|Vector|MakeVector (* _index (Variables|Default|GetDistance)) 0.0 0.0) "0,0.000000, 0")))
          (ChildActorComponent|SetChildActorClass _returnvalue "/Game/Blueprints/BridgeSystem/Trigger.Trigger_C")
          (Utilities|FlowControl|Sequence
            (:then_1
              (for _index_2 (range 1 (Math|Float|Truncate (/ (.Y (Math|Vector|BreakVector (Variables|Default|GetEnd%20Location))) (Variables|Default|GetDistance))))
                (bind _returnvalue_2 (AddComponent|AddChildActorComponent false (Math|Transform|MakeTransform (Math|Vector|MakeVector (* _index (Variables|Default|GetDistance)) (* _index_2 (Variables|Default|GetDistance)) 0.0))))
                (ChildActorComponent|SetChildActorClass _returnvalue_2 "/Game/Blueprints/BridgeSystem/Trigger.Trigger_C")))))))))