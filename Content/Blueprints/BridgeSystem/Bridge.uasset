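; Team-colored bridge segment for the pirate game mode that links to other segments and lets falling players climb onto it.
; Initialization sets team materials and registers the segment in its Root's Child list.
; Four side jump triggers send falling TestDummy characters to matching locations through a multicast climb.
; On destruction it clears its GM_Pirate status and drops children with physics and a short lifespan, cascading the collapse down the chain.
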(event OnComponentBeginOverlap(JumpTriggerB)
  (params (OtherActor :type Actor%20Object%20Reference) (OtherComp :type Primitive%20Component%20Object%20Reference) (OtherBodyIndex :type Integer) (bFromSweep :type Boolean) (SweepResult :type Hit%20Result%20Structure%20%28by%20ref%29))
  (bind _astest_dummy (Utilities|Casting|CastToTestDummy OtherActor))
  (if (AI|Components|NavMovement|IsFalling (Pawn|GetMovementComponent _astest_dummy))
    (bind _outputpin (CallFunction|TeleportPlayer _astest_dummy (Variables|Default|GetTeleLocB)))
    (Utilities|FlowControl|Delay 0.2)
    (Variables|/Game/Blueprints/TestDummy.TestDummy_C|SetisClimbing _outputpin false)))

(event OnComponentBeginOverlap(JumpTriggerL)
  (params (OtherActor :type Actor%20Object%20Reference) (OtherComp :type Primitive%20Component%20Object%20Reference) (OtherBodyIndex :type Integer) (bFromSweep :type Boolean) (SweepResult :type Hit%20Result%20Structure%20%28by%20ref%29))
  (bind _astest_dummy (Utilities|Casting|CastToTestDummy OtherActor))
  (if (AI|Components|NavMovement|IsFalling (Pawn|GetMovementComponent _astest_dummy))
    (bind _outputpin (CallFunction|TeleportPlayer _astest_dummy (Variables|Default|GetTeleLocL)))
    (Utilities|FlowControl|Delay 0.2)
    (Variables|/Game/Blueprints/TestDummy.TestDummy_C|SetisClimbing _outputpin false)))

(event OnComponentBeginOverlap(JumpTriggerR)
  (params (OtherActor :type Actor%20Object%20Reference) (OtherComp :type Primitive%20Component%20Object%20Reference) (OtherBodyIndex :type Integer) (bFromSweep :type Boolean) (SweepResult :type Hit%20Result%20Structure%20%28by%20ref%29))
  (bind _astest_dummy (Utilities|Casting|CastToTestDummy OtherActor))
  (if (AI|Components|NavMovement|IsFalling (Pawn|GetMovementComponent _astest_dummy))
    (bind _outputpin (CallFunction|TeleportPlayer _astest_dummy (Variables|Default|GetTeleLocR)))
    (Utilities|FlowControl|Delay 0.2)
    (Variables|/Game/Blueprints/TestDummy.TestDummy_C|SetisClimbing _outputpin false)))

(event OnComponentBeginOverlap(JumpTriggerF)
  (params (OtherActor :type Actor%20Object%20Reference) (OtherComp :type Primitive%20Component%20Object%20Reference) (OtherBodyIndex :type Integer) (bFromSweep :type Boolean) (SweepResult :type Hit%20Result%20Structure%20%28by%20ref%29))
  (bind _astest_dummy (Utilities|Casting|CastToTestDummy OtherActor))
  (if (AI|Components|NavMovement|IsFalling (Pawn|GetMovementComponent _astest_dummy))
    (bind _outputpin (CallFunction|TeleportPlayer _astest_dummy (Variables|Default|GetTeleLocF)))
    (Utilities|FlowControl|Delay 0.2)
    (Variables|/Game/Blueprints/TestDummy.TestDummy_C|SetisClimbing _outputpin false)))

(event Custom|SERVER%20SetStatus
  (bind _asgm_pirate (Utilities|Casting|CastToGM_Pirate (Game|GetGameMode)))
  (Default|UncheckBridgeStatus _asgm_pirate (Variables|Default|GetBridgeIndex)))

(event Custom|MULTICAST%20Initialize
  (bind _root (Variables|BridgeChaining|GetRoot))
  ;[0.2107 1 0.1084] Initialization
  (Utilities|FlowControl|Sequence
    (:then_0
      ;;[0.1476 1 0] Set Sail
      (switch Utilities|FlowControl|Switch|SwitchonTeamList (Variables|Default|GetTeamOwner)
        (:NewEnumerator0
          (Rendering|Material|SetMaterial (Variables|Components|GetBridgeMesh) 0 "/Game/Materials/MIC_Bridge_Red.MIC_Bridge_Red"))
        (:NewEnumerator1
          (Rendering|Material|SetMaterial (Variables|Components|GetFlagR) 0 "/Game/Materials/MIC_Sail_Navy.MIC_Sail_Navy")
          (Rendering|Material|SetMaterial (Variables|Components|GetFlagL) 0 "/Game/Materials/MIC_Sail_Navy.MIC_Sail_Navy")
          (Rendering|Material|SetMaterial (Variables|Components|GetBridgeMesh) 0 "/Game/Materials/MIC_Bridge_Blue.MIC_Bridge_Blue"))))
    (:then_1
      ;;[0.1699 1 0.2554] SetChild
      (Utilities|IsValid _root
        (:Is%20Valid
          (Utilities|Array|Add (Variables|Bridge_C|GetChild _root) self))))))

(event Custom|MULTICAST%20BridgeFall
  ;[1 0 0.008451] Events On Destroyed
  (Physics|SetSimulatePhysics (Variables|Components|GetBridgeMesh) true)
  (Components|DestroyComponent (Variables|Components|GetJumpTriggerF)))

(event Custom|MULTICAST%20DestroyChild
  (bind _child (Variables|BridgeChaining|GetChild))
  ;[1 0 0.008451] Events On Destroyed
  (if (!= (Utilities|Array|Length _child) 0)
    (for _array_element _child
      (Actor|SetLifeSpan _array_element 1.0)
      (CallFunction|MULTICASTBridgeFall _array_element))))

(event EventEndPlay
  (params (EndPlayReason :type EEndPlayReason%20Enum :default "Destroyed"))
  (switch Utilities|FlowControl|Switch|SwitchonEEndPlayReason EndPlayReason
    (:Destroyed
      (CallFunction|SERVERSetStatus)
      (CallFunction|MULTICASTDestroyChild))))

(fn ConstructionScript)

(fn TeleportPlayer
  (params (TestDummyReference :type Test%20Dummy%20Object%20Reference) (TeleLocation :type Scene%20Component%20Object%20Reference))
  (Default|MULTICASTClimbing TestDummyReference (Transformation|GetWorldLocation TeleLocation))
  (return TestDummyReference))