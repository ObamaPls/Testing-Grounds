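; KillZ is a level actor that kills players entering its death trigger and also handles team joining.
; On BeginPlay it copies Red, Blue and Spectator spawn locations to GS_Pirate as respawn points for deaths outside the KillZ.
; The death overlap calls DeathServer through its Server event and sets the PlayerState respawn location by team.
; JoinRed and JoinBlue triggers assign teams and move pawns to spawn, while construction-script billboards mark all three locations.
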(event OnComponentBeginOverlap(DeathTrigger)
  (params (OtherActor :type Actor%20Object%20Reference) (OtherComp :type Primitive%20Component%20Object%20Reference) (OtherBodyIndex :type Integer) (bFromSweep :type Boolean) (SweepResult :type Hit%20Result%20Structure%20%28by%20ref%29))
  ;[1 1 1] Calling the death function in the player pawn and setting the respawn point based on the player's team
  (bind _astest_dummy (Utilities|Casting|CastToTestDummy OtherActor))
  (Variables|/Game/Blueprints/TestDummy.TestDummy_C|SetDeathByKillZ _astest_dummy true)
  (Default|DestroyAllWidgets _astest_dummy)
  (CallFunction|Server (Variables|/Script/Engine.Pawn|GetPlayerState _astest_dummy) _astest_dummy))

(event OnComponentBeginOverlap(JoinRed)
  (params (OtherActor :type Actor%20Object%20Reference) (OtherComp :type Primitive%20Component%20Object%20Reference) (OtherBodyIndex :type Integer) (bFromSweep :type Boolean) (SweepResult :type Hit%20Result%20Structure%20%28by%20ref%29))
  ;[1 1 1] Putting team joining here because it's easier to manage the respawn variables
  (bind _astest_dummy (Utilities|Casting|CastToTestDummy OtherActor))
  (bind _asplayer_state_test (Utilities|Casting|CastToPlayerStateTest (Variables|/Script/Engine.Pawn|GetPlayerState _astest_dummy)))
  (Variables|/Game/Blueprints/Core/PlayerStateTest.PlayerStateTest_C|SetTeam _asplayer_state_test "NewEnumerator0")
  (Default|JoinTeam _astest_dummy)
  (Transformation|SetActorLocation _astest_dummy (Variables|Default|GetRedSpawnLocation) false false))

(event OnComponentBeginOverlap(JoinBlue)
  (params (OtherActor :type Actor%20Object%20Reference) (OtherComp :type Primitive%20Component%20Object%20Reference) (OtherBodyIndex :type Integer) (bFromSweep :type Boolean) (SweepResult :type Hit%20Result%20Structure%20%28by%20ref%29))
  ;[1 1 1] Putting team joining here because it's easier to manage the respawn variables
  (bind _astest_dummy (Utilities|Casting|CastToTestDummy OtherActor))
  (bind _asplayer_state_test (Utilities|Casting|CastToPlayerStateTest (Variables|/Script/Engine.Pawn|GetPlayerState _astest_dummy)))
  (Variables|/Game/Blueprints/Core/PlayerStateTest.PlayerStateTest_C|SetTeam _asplayer_state_test "NewEnumerator1")
  (Default|JoinTeam _astest_dummy)
  (Transformation|SetActorLocation _astest_dummy (Variables|Default|GetBlueSpawnLocation) false false))

(event Custom|Server
  (params (PlayerStateReference :type Object%20Object%20Reference) (TesstDummyReference :type Test%20Dummy%20Object%20Reference))
  ;[1 1 1] Calling the death function in the player pawn and setting the respawn point based on the player's team
  (bind _asplayer_state_test (Utilities|Casting|CastToPlayerStateTest PlayerStateReference))
  (Default|Death(Server) TesstDummyReference)
  (switch Utilities|FlowControl|Switch|SwitchonTeamList (Variables|/Game/Blueprints/Core/PlayerStateTest.PlayerStateTest_C|GetTeam _asplayer_state_test)
    (:NewEnumerator0
      (Variables|/Game/Blueprints/Core/PlayerStateTest.PlayerStateTest_C|SetRespawnLocation _asplayer_state_test (Variables|Default|GetRedSpawnLocation)))
    (:NewEnumerator1
      (Variables|/Game/Blueprints/Core/PlayerStateTest.PlayerStateTest_C|SetRespawnLocation _asplayer_state_test (Variables|Default|GetBlueSpawnLocation)))
    (:NewEnumerator2
      (Variables|/Game/Blueprints/Core/PlayerStateTest.PlayerStateTest_C|SetRespawnLocation _asplayer_state_test (Variables|Default|GetSpectatorSpawnLocation)))))

(event EventBeginPlay
  ;[1 1 1] Setting the respawn location for if the player dies without touching the KillZ
  (bind _asgs_pirate (Utilities|Casting|CastToGS_Pirate (Game|GetGameState))) ; need to use GameState because if PlayerState, need to pick a specific player state
  (Variables|/Game/Blueprints/Core/GS_Pirate.GS_Pirate_C|SetRedRespawnLocation _asgs_pirate (Variables|Default|GetRedSpawnLocation))
  (Variables|/Game/Blueprints/Core/GS_Pirate.GS_Pirate_C|SetBlueRespawnLocation _asgs_pirate (Variables|Default|GetBlueSpawnLocation))
  (Variables|/Game/Blueprints/Core/GS_Pirate.GS_Pirate_C|SetSpecRespawnLocation _asgs_pirate (Variables|Default|GetSpectatorSpawnLocation)))

(fn ConstructionScript
  (AddComponent|AddBillboardComponent false (Math|Conversions|ToTransform(Vector) (Variables|Default|GetRedSpawnLocation)))
  (AddComponent|AddBillboardComponent false (Math|Conversions|ToTransform(Vector) (Variables|Default|GetBlueSpawnLocation)))
  (AddComponent|AddBillboardComponent false (Math|Conversions|ToTransform(Vector) (Variables|Default|GetSpectatorSpawnLocation))))