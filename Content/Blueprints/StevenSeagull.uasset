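; Seagull actor that flies a Test component along a randomly generated spline path in a continuous loop.
; The construction script sizes the Area box and, when GeneratePath is set, rolls random Locations around the actor, then feeds them to the spline.
; A timeline played from Tick moves Test at constant velocity, aiming it slightly ahead along the spline, and restarts when finished.
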(event EventTick
  (params (DeltaSeconds :type Float%20%28single-precision%29))
  (bind _spline (Variables|Default|GetSpline))
  (bind _alpha_01 (Timeline|StevenSeagull Play)
    (:Update
      (Transformation|SetWorldLocationAndRotation (Variables|Default|Gettest) (Spline|GetLocationatTime _spline _alpha_01 "World" true) (Math|Rotator|FindLookatRotation (Spline|GetLocationatTime _spline _alpha_01 "World" true) (Spline|GetLocationatTime _spline (+ _alpha_01 0.02) "World" true)) false false))
    (:Finished
      (Variables|Default|SetLocationIndex (+ (Variables|Default|GetLocationIndex) 1))
      (Timeline|StevenSeagull PlayFromStart))))

(fn ConstructionScript
  (bind _returnvalue (Transformation|GetActorLocation))
  (bind _size (Variables|Default|GetSize))
  (bind _size_2 (Variables|Default|GetSize))
  (Components|Box|SetBoxExtent (Variables|Default|GetArea) (Math|Vector|MakeVector _size _size 2e+01) true)
  (if (Variables|Default|GetGenerate%20Path)
    (Utilities|Array|Clear (Variables|Default|GetLocations))
    (for _index (range 1 (Variables|Default|GetNumberOfPoints))
      (Utilities|Array|SetArrayElem (Variables|Default|GetLocations) _index (Math|Random|RandomPointinBoundingBox _returnvalue (Math|Vector|MakeVector _size_2 _size_2 (.Z (Math|Vector|BreakVector _returnvalue)))) true)
      (Variables|Default|SetGenerate%20Path false)))
  (Spline|SetSplinePoints (Variables|Default|GetSpline) (Variables|Default|GetLocations) "World"))