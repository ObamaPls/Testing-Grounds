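; ObjectiveFlag is a team objective shown as a two-part chest, colored red or blue by its Red flag.
; The construction script puts a shared dynamic material instance on the cover and lower box and tints its Albedo, which BeginPlay reapplies.
; Hide and unhide events toggle visibility and swap both meshes between two custom collision object channels.
; BeginPlay holds the visible chest on the hidden-state channel briefly before switching it.
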(event Custom|SetRedColor
  (Rendering|Material|SetVectorParameterValue (Variables|Default|GetDynamicMateriaInstance%20%28Objective%20Flag%29) "Albedo" "(R=0.700000,G=0.065253,B=0.011718,A=1.000000)" :!class /Script/Engine.MaterialInstanceDynamic))

(event Custom|SetBlueColor
  (Rendering|Material|SetVectorParameterValue (Variables|Default|GetDynamicMateriaInstance%20%28Objective%20Flag%29) "Albedo" "(R=0.067113,G=0.063577,B=0.700000,A=1.000000)" :!class /Script/Engine.MaterialInstanceDynamic))

(event Custom|HideFlag
  (Utilities|Hide/Unhide false "ECC_GameTraceChannel3"))

(event Custom|UnhideFlag
  (Utilities|Hide/Unhide true "ECC_GameTraceChannel2"))

(event EventBeginPlay
  (Utilities|Hide/Unhide true "ECC_GameTraceChannel3")
  (Utilities|FlowControl|Delay 0.7)
  (Utilities|Hide/Unhide true "ECC_GameTraceChannel2")
  (if (Variables|Default|GetRed?)
    (CallFunction|SetRedColor)
    (else
      (CallFunction|SetBlueColor))))

(fn ConstructionScript
  (Utilities|FlowControl|Sequence
    (:then_0
      (bind _returnvalue (Rendering|Material|CreateDynamicMaterialInstance "/Game/Materials/ChestMaterial.ChestMaterial" :!class /Script/Engine.KismetMaterialLibrary))
      (Variables|Default|SetDynamicMateriaInstance%20%28Objective%20Flag%29 _returnvalue)
      (Rendering|Material|SetMaterial (Variables|Default|GetLowerBoxOfChest) 0 _returnvalue)
      (Rendering|Material|SetMaterial (Variables|Default|GetCover) 0 _returnvalue))
    (:then_1
      (if (Variables|Default|GetRed?)
        (Rendering|Material|SetVectorParameterValue _returnvalue "Albedo" "(R=0.700000,G=0.065253,B=0.011718,A=1.000000)" :!class /Script/Engine.MaterialInstanceDynamic)
        (else
          (Rendering|Material|SetVectorParameterValue _returnvalue "Albedo" "(R=0.067113,G=0.063577,B=0.700000,A=1.000000)" :!class /Script/Engine.MaterialInstanceDynamic))))))