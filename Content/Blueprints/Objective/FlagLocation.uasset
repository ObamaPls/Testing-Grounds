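; FlagLocation is a team base for a capture-the-flag objective, serving as both flag spawn and drop-off point.
; On BeginPlay a server event spawns an attached ObjectiveFlag with its Red flag set from WhatTeam.
; Overlapping CaptureArea triggers a server check: a same-team TestDummy carrying a flag unhides that flag, drops carry state and scores for its team.
; The construction script tints the DropFlagHere text by team.
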(event OnComponentBeginOverlap(CaptureArea)
  (params (OtherActor :type Actor%20Object%20Reference) (OtherComp :type Primitive%20Component%20Object%20Reference) (OtherBodyIndex :type Integer) (bFromSweep :type Boolean) (SweepResult :type Hit%20Result%20Structure%20%28by%20ref%29))
  (bind _astest_dummy (Utilities|Casting|CastToTestDummy OtherActor))
  (bind _asplayer_state_test (Utilities|Casting|CastToPlayerStateTest (Variables|/Script/Engine.Pawn|GetPlayerState _astest_dummy)))
  (CallFunction|FlagCapture(Server)))

(event Custom|SpawnChest%20%28Server%29
  (CallFunction|SpawnChestFunction (Variables|Default|GetWhatTeam?)))

(event Custom|FlagCapture%20%28Server%29
  (if (and (Utilities|Enum|Equal(Enum) (Variables|/Game/Blueprints/Core/PlayerStateTest.PlayerStateTest_C|GetTeam (stale OnComponentBeginOverlap(CaptureArea) _asplayer_state_test)) (Variables|Default|GetWhatTeam?)) (Variables|/Game/Blueprints/TestDummy.TestDummy_C|GetHasFlag? (stale OnComponentBeginOverlap(CaptureArea) _astest_dummy)))
    (Default|UnhideFlag (Variables|/Game/Blueprints/TestDummy.TestDummy_C|GetFlagReference (stale OnComponentBeginOverlap(CaptureArea) _astest_dummy)))
    (Variables|/Game/Blueprints/TestDummy.TestDummy_C|SetHasFlag? (stale OnComponentBeginOverlap(CaptureArea) _astest_dummy) false)
    (Default|AddScore(Server) (stale OnComponentBeginOverlap(CaptureArea) _astest_dummy) (Variables|/Game/Blueprints/Core/PlayerStateTest.PlayerStateTest_C|GetTeam (stale OnComponentBeginOverlap(CaptureArea) _asplayer_state_test)))
    (Default|HideDummyFlag(Server) (stale OnComponentBeginOverlap(CaptureArea) _astest_dummy))))

(event EventBeginPlay
  (CallFunction|SpawnChest(Server)))

(fn ConstructionScript
  (Rendering|Components|TextRender|SetTextRenderColor (Variables|Default|GetDrop%20Flag%20Here) (Utilities|Select :Index (Variables|Default|GetWhatTeam?) :NewEnumerator0 (Math|Color|MakeColor 0 0 255 255) :NewEnumerator1 (Math|Color|MakeColor 255 0 0 255) :NewEnumerator2 (Math|Color|MakeColor 255 255 255 255))))

(fn SpawnChestFunction
  (params (TeamList :type TeamList%20Enum))
  (bind _returnvalue (Game|SpawnActorfromClass "/Game/Blueprints/Objective/ObjectiveFlag.ObjectiveFlag_C" (Variables|Default|GetFlagLocation) "Undefined" 0 0))
  (Variables|Default|SetFlagReference _returnvalue)
  (Class|SceneComponent|Attachto (Variables|/Game/Blueprints/Objective/ObjectiveFlag.ObjectiveFlag_C|GetROOT _returnvalue) (Variables|Default|GetRoot) "None" "KeepRelativeOffset" true)
  (Variables|/Game/Blueprints/Objective/ObjectiveFlag.ObjectiveFlag_C|SetRed? _returnvalue (Utilities|Select :Index TeamList :NewEnumerator0 true :NewEnumerator1 false :NewEnumerator2 false)))