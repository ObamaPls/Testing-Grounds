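; Flag objective Blueprint with chest-like parts, tinted red or blue by its Red boolean.
; The construction script creates a dynamic instance of ChestMaterial, stores it, applies it to the LowerBox and Cover meshes, and sets its Albedo parameter to the chosen color.
; BeginPlay sets the same color again on the stored instance; the file contains no capture or scoring logic.
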(event EventBeginPlay
  (bind _dynamicmaterialinstance (Variables|Default|GetDynamicMaterialInstance))
  (if (Variables|Default|GetRed?)
    (Rendering|Material|SetVectorParameterValue _dynamicmaterialinstance "Albedo" "(R=0.701961,G=0.062745,B=0.007843,A=1.000000)" :!class /Script/Engine.MaterialInstanceDynamic)
    (else
      (Rendering|Material|SetVectorParameterValue _dynamicmaterialinstance "Albedo" "(R=0.066667,G=0.062745,B=0.701961,A=1.000000)" :!class /Script/Engine.MaterialInstanceDynamic))))

(fn ConstructionScript
  (Utilities|FlowControl|Sequence
    (:then_0
      (bind _returnvalue (Rendering|Material|CreateDynamicMaterialInstance "/Game/Materials/DebugMaterials/ChestMaterial.ChestMaterial" :!class /Script/Engine.KismetMaterialLibrary))
      (Variables|Default|SetDynamicMaterialInstance _returnvalue)
      (Rendering|Material|SetMaterial (Variables|Default|GetLowerBox) 0 _returnvalue)
      (Rendering|Material|SetMaterial (Variables|Default|GetCover) 0 _returnvalue))
    (:then_1
      (if (Variables|Default|GetRed?)
        (Rendering|Material|SetVectorParameterValue _returnvalue "Albedo" "(R=0.701961,G=0.062745,B=0.007843,A=1.000000)" :!class /Script/Engine.MaterialInstanceDynamic)
        (else
          (Rendering|Material|SetVectorParameterValue _returnvalue "Albedo" "(R=0.066667,G=0.062745,B=0.701961,A=1.000000)" :!class /Script/Engine.MaterialInstanceDynamic))))))