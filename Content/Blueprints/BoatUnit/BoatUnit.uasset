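; BoatUnit is a boat actor that travels in a straight line and can sink out of the world.
; The construction script sets the ProjectileMovement velocity along the Y axis from the Speed variable.
; The Sink event stores the current location, then plays the GoDown timeline, which nudges the root downward by a fixed step each update and destroys the actor when finished.
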(event Custom|Sink
  (Variables|Default|SetActorCurrentLocation (Transformation|GetActorLocation))
  (Timeline|GoDown PlayFromStart
    (:Update
      (Transformation|AddWorldOffset (Variables|Default|GetRoot) "0, 0,-5.000000" false false))
    (:Finished
      (Actor|DestroyActor))))

(fn ConstructionScript
  (Variables|/Script/Engine.MovementComponent|SetVelocity (Variables|Default|GetProjectileMovement) (Math|Vector|MakeVector 0.0 (Variables|Default|GetSpeed) 0.0)))