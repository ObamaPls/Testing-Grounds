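; TileRailings is a Blueprint actor that tiles railing meshes in a straight row.
; Its construction script adds an instanced static mesh component and places RailingCount instances in world space, spaced by RailingLength and starting one step from the actor's location.
; Flip selects world Y or X as the row axis, while each instance copies the actor's rotation and scale.
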(fn ConstructionScript
  (bind _railinglength (Variables|Tiling|GetRailingLength))
  (bind _returnvalue (AddComponent|AddInstancedStaticMeshComponent false))
  (for _index (range 1 (Variables|Tiling|GetRailingCount))
    (Class|InstancedStaticMeshComponent|AddInstanceWorldSpace _returnvalue (Math|Transform|MakeTransform (+ (Transformation|GetActorLocation) (* (Math|Vector|SelectVector (Math|Vector|MakeVector 0.0 _railinglength 0.0) (Math|Vector|MakeVector _railinglength 0.0 0.0) (Variables|Tiling|GetFlip)) _index)) (Transformation|GetActorRotation) (Transformation|GetActorScale3D)))))