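; Boat spawner actor that periodically creates small or medium boats along a start line and destroys them at an end box.
; A looping timer, its interval randomized once at BeginPlay, calls a server event that picks boat type and X offset, then spawns through GM_Pirate.
; The construction script sizes and places both boxes from Length, Distance and UseX, though spawn positions always vary along X.
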(event OnComponentBeginOverlap(SpawnEndLocation)
  (params (OtherActor :type Actor%20Object%20Reference) (OtherComp :type Primitive%20Component%20Object%20Reference) (OtherBodyIndex :type Integer) (bFromSweep :type Boolean) (SweepResult :type Hit%20Result%20Structure%20%28by%20ref%29))
  (Utilities|Casting|CastToBoatUnit OtherActor)
  (Actor|DestroyActor OtherActor))

(event Custom|SERVER_SpawnBoat
  (bind _spawnstartlocation (Variables|Default|GetSpawnStartLocation))
  (bind _length (Variables|Spawner|GetLength))
  (bind _returnvalue (Transformation|GetWorldLocation _spawnstartlocation))
  (bind (_x _y _z) (Math|Vector|BreakVector _returnvalue))
  (bind _output_get (Variables|Default|SetSpawnTransform (Math|Transform|MakeTransform (Math|Vector|MakeVector (Math|Random|RandomFloatinRange (- _x _length) (+ _x _length)) _y _z) "0,0.000000, 0")))
  (CallFunction|SpawnRandomizer)
  (bind _asgm_pirate (Utilities|Casting|CastToGM_Pirate (Game|GetGameMode)))
  (Default|BoatSpawn _asgm_pirate (Variables|Default|GetBoatType) _output_get))

(event Custom|MULTICAST_SpawnBoat
  (params (Boat%20Type :type Actor%20Class%20Reference) (SpawnTransform :type Transform))
  (Game|SpawnActorfromClass Boat%20Type SpawnTransform "AlwaysSpawn" 0 0))

(event EventBeginPlay
  (Utilities|Time|SetTimerbyFunctionName 0 "CallForSpawn" (Math|Random|RandomFloatinRange (Variables|Spawner|GetMinTime) (Variables|Spawner|GetMaxTime)) true))

(fn ConstructionScript
  (bind _spawnendlocation (Variables|Default|GetSpawnEndLocation))
  (bind _length (Variables|Spawner|GetLength))
  (bind _distance (Variables|Spawner|GetDistance))
  (bind _length_2 (Variables|Spawner|GetLength))
  (Components|Box|SetBoxExtent (Variables|Default|GetSpawnStartLocation) (Math|Vector|SelectVector (Math|Vector|MakeVector _length_2 1e+01 1e+01) (Math|Vector|MakeVector 1e+01 _length_2 1e+01) (Variables|Spawner|GetUse%20X)) true)
  (Transformation|SetRelativeLocation _spawnendlocation (Math|Vector|SelectVector (Math|Vector|MakeVector 0.0 _distance 0.0) (Math|Vector|MakeVector _distance 0.0 0.0) (Variables|Spawner|GetUse%20X)) false false)
  (Components|Box|SetBoxExtent _spawnendlocation (Math|Vector|SelectVector (Math|Vector|MakeVector _length 1e+01 1e+01) (Math|Vector|MakeVector 1e+01 _length 1e+01) (Variables|Spawner|GetUse%20X)) true))

(fn SpawnRandomizer
  (Utilities|FlowControl|Sequence
    (:then_0
      (switch int (Math|Random|RandomInteger 2)
        (:0
          (Variables|Default|SetBoatType "/Game/Blueprints/BoatUnit_Medium.BoatUnit_Medium_C"))
        (:1
          (Variables|Default|SetBoatType "/Game/Blueprints/BoatUnit_Small.BoatUnit_Small_C"))))
    (:then_1
      (return))))

(fn CallforSpawn
  (CallFunction|SERVERSpawnBoat))