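; DeathZ is a death zone that teleports any TestDummy entering its DeathTrigger to a spawn point for its Red, Blue or Spectator team.
; The team comes from PlayerStateTest, and the construction script positions the three spawn components from relative location variables.
; For flag carriers it gathers FlagLocation actors, but the UnhideFlag call meant to restore a team-indexed flag is disconnected and never runs.
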(event OnComponentBeginOverlap(DeathTrigger)
  (params (OtherActor :type Actor%20Object%20Reference) (OtherComp :type Primitive%20Component%20Object%20Reference) (OtherBodyIndex :type Integer) (bFromSweep :type Boolean) (SweepResult :type Hit%20Result%20Structure%20%28by%20ref%29))
  ;[1 1 1] Respawning
  (bind _astest_dummy (Utilities|Casting|CastToTestDummy OtherActor))
  (bind _asplayer_state_test (Utilities|Casting|CastToPlayerStateTest (Variables|/Script/Engine.Pawn|GetPlayerState _astest_dummy)))
  (Transformation|SetActorLocation _astest_dummy (Transformation|GetWorldLocation (Utilities|Select :Index (Variables|/Game/Blueprints/Core/PlayerStateTest.PlayerStateTest_C|GetTeam _asplayer_state_test) :NewEnumerator0 (Variables|Default|GetRedSpawnLoc) :NewEnumerator1 (Variables|Default|GetBlueSpawnLoc) :NewEnumerator2 (Variables|Default|GetSpectatorSpawnLoc))) false true)
  (if (Variables|/Game/Blueprints/TestDummy.TestDummy_C|GetHasFlag? _astest_dummy)
    (bind _outactors (Actor|GetAllActorsOfClass "/Game/Blueprints/Objective/FlagLocation.FlagLocation_C"))))

(fn ConstructionScript
  (Transformation|SetRelativeLocation (Variables|Default|GetBlueSpawnLoc) (Variables|Default|GetBlueRespawnLocation) false false)
  (Transformation|SetRelativeLocation (Variables|Default|GetRedSpawnLoc) (Variables|Default|GetRedRespawnLocation) false false)
  (Transformation|SetRelativeLocation (Variables|Default|GetSpectatorSpawnLoc) (Variables|Default|GetSpectatorRespawnLocation) false false))