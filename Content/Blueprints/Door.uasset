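; A door actor that opens the boat attack by shattering on cue, with a visible numeric countdown before it.
; StartCountdown shows the Countdown text with the given number and plays a bell.
; PlaySound plays the door-open and pirate battlecry sounds, tells every DynamicBoatSpawner to start spawning boats, then destroys the door.
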(event Custom|StartCountdown
  (params (Number :type Integer%20%28by%20ref%29))
  (bind _countdown (Variables|Default|GetCountdown))
  (Rendering|SetVisibility _countdown true false)
  (Rendering|Components|TextRender|SetText _countdown (Utilities|Text|ToText(Integer) Number))
  (Audio|PlaySoundatLocation "/Game/Sounds/Countdown_Bell.Countdown_Bell" (Transformation|GetActorLocation)))

(event Custom|DestroyDoor
  (Actor|DestroyActor))

(event Custom|PlaySound
  (bind _returnvalue (Transformation|GetActorLocation))
  (Audio|PlaySoundatLocation "/Game/Sounds/OpenDoorSound.OpenDoorSound" _returnvalue)
  (Audio|PlaySoundatLocation "/Game/Sounds/Pirate_Battlecry.Pirate_Battlecry" _returnvalue)
  (bind _outactors (Actor|GetAllActorsOfClass "/Game/Blueprints/BoatUnit/DynamicBoatSpawner.DynamicBoatSpawner_C"))
  (for _array_element _outactors
    (Default|StartSpawningBoats _array_element))
  (CallFunction|DestroyDoor))

(fn ConstructionScript)